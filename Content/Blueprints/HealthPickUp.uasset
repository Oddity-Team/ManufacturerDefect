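; Health pickup that heals an overlapping SideScrollerCharacter with fewer lives than its maximum, then plays the Heal sound event and destroys itself.
; It calls UpdateHealth on the character's health reference, then sets delays on two scene light components using missing-health math expressions, the second named with a 0.4 offset.
; On destruction it adds itself to the game mode's LevelSaveData list of destroyed actors.
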(event EventDestroyed
  (bind _asside_scroller_game_mode (Utilities|Casting|CastToSideScrollerGameMode (Game|GetGameMode)))
  (Utilities|Array|Add (Variables|/Game/Blueprints/Save/SaveLevelData.SaveLevelData_C|GetActorsDestroyed (Variables|/Game/SideScrollerCPP/Blueprints/SideScrollerGameMode.SideScrollerGameMode_C|GetLevelSaveData _asside_scroller_game_mode)) (Utilities|ResolveSoftReference self)))

(event Collision|EventActorBeginOverlap
  (params (OtherActor :type Actor%20Object%20Reference))
  (bind _asside_scroller_character (Utilities|Casting|CastToSideScrollerCharacter OtherActor))
  (if (< (Variables|/Game/SideScrollerCPP/Blueprints/Widgets/HealthBar.HealthBar_C|GetLives (Variables|/Game/SideScrollerCPP/Blueprints/SideScrollerCharacter.SideScrollerCharacter_C|GetHealthRef _asside_scroller_character)) (Variables|/Game/SideScrollerCPP/Blueprints/Widgets/HealthBar.HealthBar_C|GetMaxLives (Variables|/Game/SideScrollerCPP/Blueprints/SideScrollerCharacter.SideScrollerCharacter_C|GetHealthRef _asside_scroller_character)))
    (Default|UpdateHealth (Variables|/Game/SideScrollerCPP/Blueprints/SideScrollerCharacter.SideScrollerCharacter_C|GetHealthRef _asside_scroller_character) (Variables|/Game/SideScrollerCPP/Blueprints/Widgets/HealthBar.HealthBar_C|GetLives (Variables|/Game/SideScrollerCPP/Blueprints/SideScrollerCharacter.SideScrollerCharacter_C|GetHealthRef _asside_scroller_character)) false)
    (Class|SceneLightComponent|SetDelay (Variables|/Game/SideScrollerCPP/Blueprints/SideScrollerCharacter.SideScrollerCharacter_C|GetMySceneLightComponent _asside_scroller_character) (|((MaxHealth-Health)/MaxHealth) (Math|Conversions|ToFloat(Integer) (Variables|/Game/SideScrollerCPP/Blueprints/Widgets/HealthBar.HealthBar_C|GetMaxLives (Variables|/Game/SideScrollerCPP/Blueprints/SideScrollerCharacter.SideScrollerCharacter_C|GetHealthRef _asside_scroller_character))) (Math|Conversions|ToFloat(Integer) (Variables|/Game/SideScrollerCPP/Blueprints/Widgets/HealthBar.HealthBar_C|GetLives (Variables|/Game/SideScrollerCPP/Blueprints/SideScrollerCharacter.SideScrollerCharacter_C|GetHealthRef _asside_scroller_character)))))
    (Class|SceneLightComponent|SetDelay (Variables|/Game/SideScrollerCPP/Blueprints/SideScrollerCharacter.SideScrollerCharacter_C|GetMySceneLightComponent1 _asside_scroller_character) (|((((MaxHealth-Health)/MaxHealth)-0.400000)*1) (Math|Conversions|ToFloat(Integer) (Variables|/Game/SideScrollerCPP/Blueprints/Widgets/HealthBar.HealthBar_C|GetMaxLives (Variables|/Game/SideScrollerCPP/Blueprints/SideScrollerCharacter.SideScrollerCharacter_C|GetHealthRef _asside_scroller_character))) (Math|Conversions|ToFloat(Integer) (Variables|/Game/SideScrollerCPP/Blueprints/Widgets/HealthBar.HealthBar_C|GetLives (Variables|/Game/SideScrollerCPP/Blueprints/SideScrollerCharacter.SideScrollerCharacter_C|GetHealthRef _asside_scroller_character)))))
    (Class|FMODBlueprintStatics|PlayEvent2D "/Game/FMOD/Events/Heal.Heal")
    (Actor|DestroyActor)))

(fn ConstructionScript)