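; TeleportPortal_BP is a two-way teleport portal that moves a SideScrollerCharacter between linked portals.
; On Hit by that character, it plays a falling sound and searches all portal actors for one with the same PortalIndex and opposite Entrance flag.
; It then moves the character to that partner's Exit location.
; The construction script positions the Portal and Exit components from variables.
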(event EventBeginPlay)

(event Collision|EventActorBeginOverlap
  (params (OtherActor :type Actor%20Object%20Reference)))

(event EventTick
  (params (DeltaSeconds :type Float%20%28single-precision%29)))

(event Collision|EventHit
  (params (MyComp :type Primitive%20Component%20Object%20Reference) (Other :type Actor%20Object%20Reference) (OtherComp :type Primitive%20Component%20Object%20Reference) (bSelfMoved :type Boolean) (HitLocation :type Vector :default "0, 0, 0") (HitNormal :type Vector :default "0, 0, 0") (NormalImpulse :type Vector :default "0, 0, 0") (Hit :type Hit%20Result%20Structure%20%28by%20ref%29))
  (bind _asside_scroller_character (Utilities|Casting|CastToSideScrollerCharacter Other))
  (Audio|PlaySound2D "/Game/Interface_And_Item_Sounds/WAV/Cartoon_Falling_02.Cartoon_Falling_02" 1.0 1.0 0.0 0 0)
  (if (Variables|Default|GetEntrance?)
    (bind _outactors (Actor|GetAllActorsOfClass "TeleportPortal_BP_C"))
    (bind _array_element (Utilities|Array|ForEachLoopwithBreak _outactors :!label _label)
      (:LoopBody
        (if (and (== (Variables|TeleportPortal_BP_C|GetPortalIndex _array_element) (Variables|Default|GetPortalIndex)) (not (Variables|TeleportPortal_BP_C|GetEntrance? _array_element)))
          (goto _label Break)))
      (:Completed
        (Transformation|SetActorLocation _asside_scroller_character (Transformation|GetWorldLocation (Variables|TeleportPortal_BP_C|GetExit _array_element)) false false)))
    (else
      (bind _outactors_2 (Actor|GetAllActorsOfClass "TeleportPortal_BP_C"))
      (bind _array_element_2 (Utilities|Array|ForEachLoopwithBreak _outactors_2 :!label _label_2)
        (:LoopBody
          (if (and (== (Variables|TeleportPortal_BP_C|GetPortalIndex _array_element_2) (Variables|Default|GetPortalIndex)) (and (not (Variables|Default|GetEntrance?)) (Variables|TeleportPortal_BP_C|GetEntrance? _array_element_2)))
            (goto _label_2 Break)))
        (:Completed
          (Transformation|SetActorLocation _asside_scroller_character (Transformation|GetWorldLocation (Variables|TeleportPortal_BP_C|GetExit _array_element_2)) false false))))))

(fn ConstructionScript
  (Transformation|SetRelativeTransform (Variables|Default|GetPortal) (Variables|Default|GetPortalTransform) false false)
  (Transformation|SetRelativeLocation (Variables|Default|GetExit) (Variables|Default|GetNew%20Location) false false))