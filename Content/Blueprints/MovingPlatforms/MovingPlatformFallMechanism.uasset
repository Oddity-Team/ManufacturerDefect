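; A platform that falls after a set delay once the SideScrollerCharacter overlaps its trigger box.
; A timeline lowers the platform, cube and box together and then flags it as down, while a separate timeline started on BeginPlay drives the platform's rotation.
; An Activate event, bound to a dispatcher every Tick, runs another timeline to move all three parts if down and enabled via EnableMechanism, then clears both flags.
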(event OnComponentBeginOverlap(Box)
  (params (OverlappedComponent :type Primitive%20Component%20Object%20Reference) (OtherActor :type Actor%20Object%20Reference) (OtherComp :type Primitive%20Component%20Object%20Reference) (OtherBodyIndex :type Integer) (bFromSweep :type Boolean) (SweepResult :type Hit%20Result%20Structure%20%28by%20ref%29))
  (Utilities|Casting|CastToSideScrollerCharacter OtherActor)
  (Utilities|FlowControl|Delay (Variables|Default|GetFallAfterSetSeconds))
  (Utilities|FlowControl|Sequence
    (:then_0
      (bind _fall (Timeline|Timeline_1 PlayFromStart)
        (:Update
          (Utilities|FlowControl|Sequence
            (:then_0
              (Transformation|SetRelativeLocation (Variables|Default|GetCube) (Math|Vector|MakeVector 0.0 0.0 (.z _fall)) false false))
            (:then_1
              (Transformation|SetRelativeLocation (Variables|Default|GetMoving%20Platform%20Fall) (Math|Vector|MakeVector 0.0 0.0 (.z _fall)) false false))
            (:then_2
              (Transformation|SetRelativeLocation (Variables|Default|GetBox) (Math|Vector|MakeVector 0.0 0.0 (.z _fall)) false false))))
        (:Finished
          (Variables|Default|SetDown true))))))

(event Custom|Activate
  (if (and (Variables|Default|GetEnabled) (Variables|Default|GetDown))
    (bind _z (Timeline|Timeline_3 PlayFromStart)
      (:Update
        (Utilities|FlowControl|Sequence
          (:then_0
            (Transformation|SetRelativeLocation (Variables|Default|GetMoving%20Platform%20Fall) _z false false))
          (:then_1
            (Transformation|SetRelativeLocation (Variables|Default|GetCube) _z false false))
          (:then_2
            (Transformation|SetRelativeLocation (Variables|Default|GetBox) _z false false)
            (Development|PrintString "Hello"))))
      (:Finished
        (Variables|Default|SetEnabled false)
        (Variables|Default|SetDown false)))))

(event EventBeginPlay
  (bind _rotation_z (Timeline|RotationPlatform Play)
    (:Update
      (Transformation|SetRelativeRotation (Variables|Default|GetMoving%20Platform%20Fall) (Math|Rotator|Lerp(Rotator) (Variables|Default|GetStartRotation) (Variables|Default|GetEndRotation) _rotation_z) false false))))

(event EventTick
  (params (DeltaSeconds :type Float%20%28single-precision%29))
  (EventDispatchers|BindEventtoActivateDisp (delegate Custom|Activate)))

(fn ConstructionScript)

(fn EnableMechanism
  (Variables|Default|SetEnabled true))