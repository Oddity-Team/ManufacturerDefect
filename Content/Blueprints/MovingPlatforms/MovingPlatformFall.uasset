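; Side-scroller moving platform that falls after a set delay when the player character overlaps its trigger box, then rises back.
; On overlap it plays a sound and a timeline that drives the Z location of the cube and platform components.
; A DoOnce, reset on each trigger, reverses that timeline once when it finishes.
; A separate timeline started on BeginPlay rotates the platform between start and end rotations.
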(event OnComponentBeginOverlap(Box)
  (params (OverlappedComponent :type Primitive%20Component%20Object%20Reference) (OtherActor :type Actor%20Object%20Reference) (OtherComp :type Primitive%20Component%20Object%20Reference) (OtherBodyIndex :type Integer) (bFromSweep :type Boolean) (SweepResult :type Hit%20Result%20Structure%20%28by%20ref%29))
  (Utilities|Casting|CastToSideScrollerCharacter OtherActor)
  (Utilities|FlowControl|Delay (Variables|Default|GetFallAfterSetSeconds))
  (Class|FMODBlueprintStatics|PlayEvent2D "/Game/FMOD/Events/Platform_Fall.Platform_Fall")
  (Utilities|FlowControl|Sequence
    (:then_1
      (bind _fall (Timeline|Timeline_0 Play)
        (:Update
          (Utilities|FlowControl|Sequence
            (:then_0
              (Transformation|SetRelativeLocation (Variables|Default|GetCube) (Math|Vector|MakeVector 0.0 0.0 (.z _fall)) false false))
            (:then_1
              (Transformation|SetRelativeLocation (Variables|Default|GetMoving%20Platform%20Fall) (Math|Vector|MakeVector 0.0 0.0 (.z _fall)) false false))))
        (:Finished
          (Utilities|FlowControl|DoOnce false :!label _label
            (:Completed
              (Timeline|Timeline_0 Reverse))))))
    (:then_2
      (goto _label Reset))))

(event EventBeginPlay
  (bind _rotation_z (Timeline|RotationPlatform Play)
    (:Update
      (Transformation|SetRelativeRotation (Variables|Default|GetMoving%20Platform%20Fall) (Math|Rotator|Lerp(Rotator) (Variables|Default|GetStartRotation) (Variables|Default|GetEndRotation) _rotation_z) false false))))

(fn ConstructionScript)