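; Moving platform that travels along its relative Y axis as a rotating gear, paired with a cube that follows without spinning.
; Three timelines start on BeginPlay: two set the Y location of the cube and gear, and one lerps the gear's rotation.
; The cube keeps the player from rotating and falling off, so both movement branches must stay identical.
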(event EventBeginPlay
  (Utilities|FlowControl|Sequence
    (:then_0
      ;[1 1 1] Cube Movement (so player is not rotating -> not falling off)
      ;;[1 1 1] THIS NODES MUST BE THE SAME
      (bind _height (Timeline|MovingCube PlayFromStart)
        (:Update
          (Transformation|SetRelativeLocation (Variables|Default|GetCube) (Math|Vector|MakeVector 0.0 (.y _height) 0.0) false false))))
    (:then_1
      ;[1 1 1] Gear Movement
      (bind _height_2 (Timeline|MovingPlatform PlayFromStart)
        (:Update
          (Transformation|SetRelativeLocation (Variables|Default|GetMoving%20Platform) (Math|Vector|MakeVector 0.0 (.y _height_2) 0.0) false false))))
    (:then_2
      ;[1 1 1] Gear Rotation
      (bind _rotation_z (Timeline|RotatingPlatform PlayFromStart)
        (:Update
          (Transformation|SetRelativeRotation (Variables|Default|GetMoving%20Platform) (Math|Rotator|Lerp(Rotator) (Variables|Default|GetStartRotation) (Variables|Default|GetEndRotation) _rotation_z) false false))))))

(fn ConstructionScript)