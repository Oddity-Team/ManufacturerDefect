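; A press hazard for a side-scroller that moves its cube along a timeline and hurts characters it hits.
; Shortly after BeginPlay, unless disabled, PressLine starts driving the cube's relative location without sweeping.
; A hit side-scroller character takes damage and is launched with one of two velocities, chosen by the sign of its forward Y.
; DisableMechanism sets a flag that turns off timeline looping, so the press finishes its current cycle.
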(event EventBeginPlay
  (Utilities|FlowControl|Delay 0.2)
  (if (not (Variables|Default|GetDisabled))
    (bind _pressloc (Timeline|PressLine PlayFromStart)
      (:Update
        (if (Variables|Default|GetDisabled)
          (Components|Timeline|SetLooping (Variables|Default|GetPressLine) false))
        (Transformation|SetRelativeLocation (Variables|Default|GetCube) _pressloc false false)))))

(event Collision|EventHit
  (params (MyComp :type Primitive%20Component%20Object%20Reference) (Other :type Actor%20Object%20Reference) (OtherComp :type Primitive%20Component%20Object%20Reference) (bSelfMoved :type Boolean) (HitLocation :type Vector :default "0, 0, 0") (HitNormal :type Vector :default "0, 0, 0") (NormalImpulse :type Vector :default "0, 0, 0") (Hit :type Hit%20Result%20Structure%20%28by%20ref%29))
  (bind _asside_scroller_character (Utilities|Casting|CastToSideScrollerCharacter Other))
  (Game|Damage|ApplyDamage _asside_scroller_character 1e+01 0 0)
  (if (> (.Y (Math|Vector|BreakVector (Math|Vector|GetForwardVector (Variables|/Script/Engine.Actor|GetRootComponent _asside_scroller_character)))) 0.0)
    (Character|LaunchCharacter _asside_scroller_character (Variables|Default|GetLaunch%20Velocity) false false)
    (else
      (Character|LaunchCharacter _asside_scroller_character (Variables|Default|GetLaunch%20Velocity%201) false false))))

(fn ConstructionScript)

(fn DisableMechanism
  (Variables|Default|SetDisabled true))