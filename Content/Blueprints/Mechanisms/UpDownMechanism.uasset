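; Lift mechanism that moves a platform between up and down positions when activated.
; Each Tick rebinds Activate to an ActivateDisp dispatcher, and Activate runs only while Enabled, which EnableMechanism sets.
; The Up and Down flags select the DownMovement or UpMovement timeline, which sets the platform's relative location and fires a Lift sound every update.
; Finishing a move swaps the flags and clears Enabled, so another move requires re-enabling.
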(event Custom|Activate
  (if (Variables|Default|GetEnabled)
    (Utilities|FlowControl|Sequence
      (:then_0
        (if (Variables|Default|GetUp)
          (bind _z (Timeline|DownMovement PlayFromStart)
            (:Update
              (Transformation|SetRelativeLocation (Variables|Default|GetPlatform) _z false false)
              (Class|FMODBlueprintStatics|PlayEvent2D "/Game/FMOD/Events/Lift.Lift"))
            (:Finished
              (Variables|Default|SetDown true)
              (Variables|Default|SetUp false)
              (Variables|Default|SetEnabled false)))))
      (:then_1
        (if (Variables|Default|GetDown)
          (bind _z_2 (Timeline|UpMovement PlayFromStart)
            (:Update
              (Transformation|SetRelativeLocation (Variables|Default|GetPlatform) _z_2 false false)
              (Class|FMODBlueprintStatics|PlayEvent2D "/Game/FMOD/Events/Lift.Lift"))
            (:Finished
              (Variables|Default|SetUp true)
              (Variables|Default|SetDown false)
              (Variables|Default|SetEnabled false))))))))

(event EventTick
  (params (DeltaSeconds :type Float%20%28single-precision%29))
  (EventDispatchers|BindEventtoActivateDisp (delegate Custom|Activate)))

(fn ConstructionScript)

(fn EnableMechanism
  (Variables|Default|SetEnabled true))