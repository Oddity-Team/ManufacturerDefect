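; Side-scroller AI enemy with lives and a health bar widget that keeps a fixed world rotation.
; Non-top hits damage and launch the player by facing direction; a detection capsule sets IsAttacking, and DoAttack toggles the damaging attack capsule.
; Each damage event costs one life; at zero, effects play and the EnDeathFromFall dispatcher triggers FallDeath, stopping AI logic before delayed destruction.
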(event OnComponentBeginOverlap(Capsule1)
  (params (OverlappedComponent :type Primitive%20Component%20Object%20Reference) (OtherActor :type Actor%20Object%20Reference) (OtherComp :type Primitive%20Component%20Object%20Reference) (OtherBodyIndex :type Integer) (bFromSweep :type Boolean) (SweepResult :type Hit%20Result%20Structure%20%28by%20ref%29))
  (Utilities|Casting|CastToSideScrollerCharacter OtherActor)
  (Variables|Components|SetIs%20Attacking true))

(event OnComponentBeginOverlap(CapsuleCol)
  (params (OverlappedComponent :type Primitive%20Component%20Object%20Reference) (OtherActor :type Actor%20Object%20Reference) (OtherComp :type Primitive%20Component%20Object%20Reference) (OtherBodyIndex :type Integer) (bFromSweep :type Boolean) (SweepResult :type Hit%20Result%20Structure%20%28by%20ref%29))
  (bind _asside_scroller_character (Utilities|Casting|CastToSideScrollerCharacter OtherActor))
  (Game|Damage|ApplyDamage _asside_scroller_character 1.0 0 0))

(event OnComponentEndOverlap(CapsuleCol)
  (params (OverlappedComponent :type Primitive%20Component%20Object%20Reference) (OtherActor :type Actor%20Object%20Reference) (OtherComp :type Primitive%20Component%20Object%20Reference) (OtherBodyIndex :type Integer)))

(event OnComponentEndOverlap(Capsule1)
  (params (OverlappedComponent :type Primitive%20Component%20Object%20Reference) (OtherActor :type Actor%20Object%20Reference) (OtherComp :type Primitive%20Component%20Object%20Reference) (OtherBodyIndex :type Integer))
  (Utilities|Casting|CastToSideScrollerCharacter OtherActor)
  (Variables|Components|SetIs%20Attacking false))

(event Custom|FallDeath
  (AI|Logic|StopLogic (Variables|/Script/AIModule.AIController|GetBrainComponent (AI|GetAIController self)) "")
  (Utilities|FlowControl|Delay 1.5)
  (Actor|DestroyActor))

(event EventBeginPlay
  (bind _asai_health_bar (Utilities|Casting|CastToAI_HealthBar (UserInterface|GetUserWidgetObject (Variables|Default|GetHealthBar))))
  (Variables|/Game/Blueprints/AI/AI_HealthBar.AI_HealthBar_C|SetEnemy _asai_health_bar self)
  (EventDispatchers|BindEventtoEnDeathfromFall (delegate Custom|FallDeath)))

(event Game|Damage|EventAnyDamage
  (params (Damage :type Float%20%28single-precision%29) (DamageType :type Damage%20Type%20Object%20Reference) (InstigatedBy :type Controller%20Object%20Reference) (DamageCauser :type Actor%20Object%20Reference))
  (bind _output_get (Variables|Components|SetLives (- (Variables|Components|GetLives) 1)))
  (if (<= _output_get 0)
    (Audio|PlaySoundatLocation "/Game/StarterContent/Audio/Explosion01.Explosion01" "0, 0, 0" "0, 0, 0" 0.5 1.0 0.0 0 0 0)
    (Effects|SpawnEmitteratLocation "/Game/Blueprints/AI/P_Sparks_Destroy.P_Sparks_Destroy" (Transformation|GetActorLocation))
    (Default|CallEnDeathfromFall)
    (else
      (Audio|PlaySoundatLocation "/Game/Interface_And_Item_Sounds/WAV/Error_Buzz_03.Error_Buzz_03" "0, 0, 0" "0, 0, 0" 1.0 1.0 0.0 0 0 0))))

(event EventTick
  (params (DeltaSeconds :type Float%20%28single-precision%29))
  (Transformation|SetWorldRotation (Variables|Default|GetHealthBar) "0, 0, 0" false false))

(event Collision|EventHit
  (params (MyComp :type Primitive%20Component%20Object%20Reference) (Other :type Actor%20Object%20Reference) (OtherComp :type Primitive%20Component%20Object%20Reference) (bSelfMoved :type Boolean) (HitLocation :type Vector :default "0, 0, 0") (HitNormal :type Vector :default "0, 0, 0") (NormalImpulse :type Vector :default "0, 0, 0") (Hit :type Hit%20Result%20Structure%20%28by%20ref%29))
  (Utilities|FlowControl|Delay 0.1)
  (if (> (.Z (Math|Vector|BreakVector HitNormal)) -0.8)
    (bind _asside_scroller_character (Utilities|Casting|CastToSideScrollerCharacter Other))
    (Game|Damage|ApplyDamage _asside_scroller_character 1e+01 0 0)
    (if (> (.Y (Math|Vector|BreakVector (Math|Vector|GetForwardVector (Variables|/Script/Engine.Actor|GetRootComponent _asside_scroller_character)))) 0.0)
      (Character|LaunchCharacter _asside_scroller_character (Variables|Components|GetLaunch%20Velocity) false false)
      (else
        (Character|LaunchCharacter _asside_scroller_character (Variables|Components|GetLaunch%20Velocity1) false false)))))

(event Collision|EventActorBeginOverlap
  (params (OtherActor :type Actor%20Object%20Reference)))

(fn ConstructionScript)

(fn DoAttack
  (params (Is%20Attacking :type Boolean))
  (bind _capsulecol (Variables|Default|GetCapsuleCol))
  (if Is%20Attacking
    (Collision|SetCollisionEnabled _capsulecol "QueryOnly")
    (else
      (Collision|SetCollisionEnabled _capsulecol "NoCollision")
      (Variables|Components|SetIs%20Attacking false))))