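; Side-scroller object the player can push or pull along the Y axis while inside its Box trigger.
; E toggles pulling, which slows the player, locks rotation to the entry facing and steps Move opposite that facing each frame.
; Otherwise, player Y velocity only sets the pushing flag and a reduced walk speed; the script does not move the object.
; Leaving the box restores speed and clears both flags.
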(event OnComponentBeginOverlap(Box)
  (params (OverlappedComponent :type Primitive%20Component%20Object%20Reference) (OtherActor :type Actor%20Object%20Reference) (OtherComp :type Primitive%20Component%20Object%20Reference) (OtherBodyIndex :type Integer) (bFromSweep :type Boolean) (SweepResult :type Hit%20Result%20Structure%20%28by%20ref%29))
  (if (== OtherActor (Variables|Default|GetPlayerRef))
    (Variables|Default|SetTick true)
    (Variables|Default|SetActorRotation (Transformation|GetActorRotation (Variables|Default|GetPlayerRef)))
    (else
      (Variables|Default|SetTick false))))

(event OnComponentEndOverlap(Box)
  (params (OverlappedComponent :type Primitive%20Component%20Object%20Reference) (OtherActor :type Actor%20Object%20Reference) (OtherComp :type Primitive%20Component%20Object%20Reference) (OtherBodyIndex :type Integer))
  (if (== OtherActor (Variables|Default|GetPlayerRef))
    (Variables|Default|SetTick false)
    (Variables|/Script/Engine.CharacterMovementComponent|SetMaxWalkSpeed (Variables|/Script/Engine.Character|GetCharacterMovement (Variables|Default|GetPlayerRef)) 6e+02)
    (Variables|/Game/SideScrollerCPP/Blueprints/SideScrollerCharacter.SideScrollerCharacter_C|SetIsPushing (Variables|Default|GetPlayerRef) false)
    (Variables|/Game/SideScrollerCPP/Blueprints/SideScrollerCharacter.SideScrollerCharacter_C|SetIsPulling (Variables|Default|GetPlayerRef) false)))

(event EventBeginPlay
  (bind _asside_scroller_character (Utilities|Casting|CastToSideScrollerCharacter (Game|GetPlayerCharacter 0)))
  (Variables|Default|SetPlayerRef _asside_scroller_character)
  (Input|EnableInput (Game|GetPlayerController 0)))

(event Collision|EventActorBeginOverlap
  (params (OtherActor :type Actor%20Object%20Reference)))

(event EventTick
  (params (DeltaSeconds :type Float%20%28single-precision%29))
  (bind _playerref (Variables|Default|GetPlayerRef))
  (bind _move (Variables|Default|GetMove))
  (bind _playerref_2 (Variables|Default|GetPlayerRef))
  (bind _returnvalue (Transformation|GetWorldLocation _move))
  (bind _charactermovement (Variables|/Script/Engine.Character|GetCharacterMovement _playerref_2))
  (bind (_x _y _z) (Math|Vector|BreakVector _returnvalue))
  (if (Variables|Default|GetTick)
    (if (and (not (and (< (.Y (Math|Vector|BreakVector (Class|Pawn|GetLastMovementInputVector _playerref))) 0.0) (< (.Y (Math|Vector|BreakVector (Transformation|GetActorForwardVector _playerref))) 0.0))) (Variables|/Game/SideScrollerCPP/Blueprints/SideScrollerCharacter.SideScrollerCharacter_C|GetIsPulling (Variables|Default|GetPlayerRef)))
      (Variables|/Script/Engine.CharacterMovementComponent|SetMaxWalkSpeed (Variables|/Script/Engine.Character|GetCharacterMovement (Variables|Default|GetPlayerRef)) 1e+02)
      (Variables|Default|SetObjectOffset (- (.Y (Math|Vector|BreakVector (Transformation|GetWorldLocation (Variables|/Script/Engine.Character|GetMesh (Variables|Default|GetPlayerRef))))) (.Y (Math|Vector|BreakVector _returnvalue))))
      (Transformation|SetActorRotation (Variables|Default|GetPlayerRef) (Variables|Default|GetActorRotation))
      (Transformation|SetRelativeLocation (Variables|Default|GetMove) (Math|Vector|MakeVector _x (- _y (* (.Y (Math|Vector|BreakVector (Transformation|GetActorForwardVector (Variables|Default|GetPlayerRef)))) 2.0)) _z) false false)
      (else
        (Variables|/Game/SideScrollerCPP/Blueprints/SideScrollerCharacter.SideScrollerCharacter_C|SetIsPulling (Variables|Default|GetPlayerRef) false)
        (if (!= (.Y (Math|Vector|BreakVector (Variables|/Script/Engine.MovementComponent|GetVelocity (Variables|/Script/Engine.Character|GetCharacterMovement (Variables|Default|GetPlayerRef))))) 0.0)
          (Variables|/Game/SideScrollerCPP/Blueprints/SideScrollerCharacter.SideScrollerCharacter_C|SetIsPushing _playerref_2 true)
          (Variables|/Script/Engine.CharacterMovementComponent|SetMaxWalkSpeed _charactermovement 2e+02)
          (else
            (Variables|/Game/SideScrollerCPP/Blueprints/SideScrollerCharacter.SideScrollerCharacter_C|SetIsPushing _playerref_2 false)
            (Variables|/Script/Engine.CharacterMovementComponent|SetMaxWalkSpeed _charactermovement 6e+02)))))))

(event Input|KeyboardEvents|E
  (params (Key :type Key%20Structure :default "None"))
  (bind _playerref (Variables|Default|GetPlayerRef))
  (:Pressed
    (if (Variables|Default|GetTick)
      (if (not (Variables|/Game/SideScrollerCPP/Blueprints/SideScrollerCharacter.SideScrollerCharacter_C|GetIsPulling (Variables|Default|GetPlayerRef)))
        (Variables|/Game/SideScrollerCPP/Blueprints/SideScrollerCharacter.SideScrollerCharacter_C|SetIsPulling _playerref true)
        (else
          (Variables|/Game/SideScrollerCPP/Blueprints/SideScrollerCharacter.SideScrollerCharacter_C|SetIsPulling _playerref false))))))

(fn ConstructionScript)