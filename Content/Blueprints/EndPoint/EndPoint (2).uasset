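; Level end point actor for a side-scroller, triggered when the SideScrollerCharacter overlaps its Trigger.
; It shows an EndPoint widget, plays a coin sound and hides the EndPoint component, then waits out a delay.
; It then removes the widget, destroys itself and continues in the same chain to open MainMenu with InGame set, disable player movement and show the cursor.
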(event OnComponentBeginOverlap(Trigger)
  (params (OverlappedComponent :type Primitive%20Component%20Object%20Reference) (OtherActor :type Actor%20Object%20Reference) (OtherComp :type Primitive%20Component%20Object%20Reference) (OtherBodyIndex :type Integer) (bFromSweep :type Boolean) (SweepResult :type Hit%20Result%20Structure%20%28by%20ref%29))
  (Input|EnableInput (Game|GetPlayerController 0))
  (Utilities|Casting|CastToSideScrollerCharacter OtherActor)
  (bind _returnvalue (UserInterface|CreateWidget "/Game/Blueprints/UI/EndPoint.EndPoint_C" (Game|GetPlayerController 0)))
  (Variables|Default|SetEndPointWidget%20ref _returnvalue)
  (UserInterface|Viewport|AddtoViewport (Variables|Default|GetEndPointWidget%20ref) 0)
  (CallFunction|CoinPlaySound)
  (Utilities|FlowControl|Delay (Variables|Default|GetTime))
  (Widget|RemovefromParent (Variables|Default|GetEndPointWidget%20ref))
  (Actor|DestroyActor)
  (bind _returnvalue_2 (UserInterface|CreateWidget "/Game/Blueprints/UI/MainMenu.MainMenu_C" (Game|GetPlayerController 0)))
  (Variables|Default|SetMainMenuWidget%20ref _returnvalue_2)
  (Variables|/Game/Blueprints/UI/MainMenu.MainMenu_C|SetInGame (Variables|Default|GetMainMenuWidget%20ref) true)
  (UserInterface|Viewport|AddtoViewport (Variables|Default|GetMainMenuWidget%20ref) 0)
  (Pawn|Components|CharacterMovement|DisableMovement (Variables|/Script/Engine.Character|GetCharacterMovement (Game|GetPlayerCharacter 0)))
  (Variables|/Script/Engine.PlayerController|SetbShowMouseCursor (Game|GetPlayerController 0) true))

(event Custom|CoinPlaySound
  (Audio|PlaySoundatLocation "/Game/Interface_And_Item_Sounds/WAV/Coins_13.Coins_13" (Transformation|GetActorLocation) "0, 0, 0" 0.5 1.0 0.0 "/Game/Audio/NaturalAttenuation.NaturalAttenuation" 0 0)
  (Rendering|SetVisibility (Variables|Default|GetEndPoint) false false))

(fn ConstructionScript)