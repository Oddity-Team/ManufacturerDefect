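; SaveGame object that stores the player's lives, coins, last save point and level name.
; SavePlayerData copies lives and coins from the player and writes itself to its slot.
; SavePoint calls SavePlayerData, then records the save point's PlayerStartTag and the level name and saves again.
; LoadPlayerData only applies stored values to the player, passing lives into SetHealth, without reading the slot.
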(event Custom|SavePlayerData
  (params (Player :type Side%20Scroller%20Character%20Object%20Reference))
  (Variables|Default|SetPlayerLives (Variables|/Game/SideScrollerCPP/Blueprints/Widgets/HealthBar.HealthBar_C|GetLives (Variables|/Game/SideScrollerCPP/Blueprints/SideScrollerCharacter.SideScrollerCharacter_C|GetHealthRef Player)))
  (Variables|Default|SetPlayerCoins (Variables|/Game/SideScrollerCPP/Blueprints/SideScrollerCharacter.SideScrollerCharacter_C|GetCoins Player))
  (SaveGame|SaveGametoSlot self (Variables|Default|GetSlot%20Name)))

(event Custom|LoadPlayerData
  (params (Player :type Side%20Scroller%20Character%20Object%20Reference))
  (Default|SetHealth (Variables|/Game/SideScrollerCPP/Blueprints/SideScrollerCharacter.SideScrollerCharacter_C|GetHealthRef Player) (Variables|Default|GetPlayerLives))
  (Variables|/Game/SideScrollerCPP/Blueprints/SideScrollerCharacter.SideScrollerCharacter_C|SetCoins Player (Variables|Default|GetPlayerCoins)))

(event Custom|SavePoint
  (params (SavePoint :type Save%20Point%20Object%20Reference) (Player :type Side%20Scroller%20Character%20Object%20Reference) (LevelName :type Name))
  (CallFunction|SavePlayerData Player)
  (Variables|Default|SetSavePointName (Utilities|String|ToString(Name) (Variables|/Script/Engine.PlayerStart|GetPlayerStartTag SavePoint)))
  (Variables|Default|SetLevelName LevelName)
  (SaveGame|SaveGametoSlot self (Variables|Default|GetSlot%20Name)))