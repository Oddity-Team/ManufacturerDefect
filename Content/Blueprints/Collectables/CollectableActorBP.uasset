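; Collectable actor for a side-scroller that pauses the player to present a widget.
; Trigger overlap enables input, passes its Index to the character's ImageIndex, disables movement, plays the Script event in 2D and shows CollectableWidgetBP after a delay.
; Pressing T removes the widget, restores walking and destroys the actor.
; A separate CoinPlaySound event plays a sound and lightning particle, then hides the CoinGear component.
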(event OnComponentBeginOverlap(Trigger)
  (params (OverlappedComponent :type Primitive%20Component%20Object%20Reference) (OtherActor :type Actor%20Object%20Reference) (OtherComp :type Primitive%20Component%20Object%20Reference) (OtherBodyIndex :type Integer) (bFromSweep :type Boolean) (SweepResult :type Hit%20Result%20Structure%20%28by%20ref%29))
  (Input|EnableInput (Game|GetPlayerController 0))
  (bind _asside_scroller_character (Utilities|Casting|CastToSideScrollerCharacter OtherActor))
  (Variables|/Game/SideScrollerCPP/Blueprints/SideScrollerCharacter.SideScrollerCharacter_C|SetImageIndex _asside_scroller_character (Variables|Default|GetIndex))
  (Pawn|Components|CharacterMovement|DisableMovement (Variables|/Script/Engine.Character|GetCharacterMovement (Game|GetPlayerCharacter 0)))
  (bind _returnvalue (UserInterface|CreateWidget "/Game/Blueprints/UI/CollectableWidgetBP.CollectableWidgetBP_C"))
  (Variables|Default|SetWidget%20ref _returnvalue)
  (Class|FMODBlueprintStatics|PlayEvent2D "/Game/FMOD/Events/Script.Script")
  (Utilities|FlowControl|Delay (Variables|Default|GetTime))
  (UserInterface|Viewport|AddtoViewport (Variables|Default|GetWidget%20ref) 0))

(event Custom|CoinPlaySound
  (bind _returnvalue (Transformation|GetActorLocation))
  (Audio|PlaySoundatLocation "/Game/Interface_And_Item_Sounds/WAV/Back_Click_02.Back_Click_02" _returnvalue "0, 0, 0" 0.5 1.0 0.0 "/Game/Audio/NaturalAttenuation.NaturalAttenuation" 0 0)
  (Effects|SpawnEmitteratLocation "/Game/RPGEffects/Particles/P_Mage_Lightning_Bolt.P_Mage_Lightning_Bolt" _returnvalue)
  (Rendering|SetVisibility (Variables|Default|GetCoinGear) false false))

(event Input|KeyboardEvents|T
  (params (Key :type Key%20Structure :default "None"))
  (:Pressed
    (Widget|RemovefromParent (Variables|Default|GetWidget%20ref))
    (Pawn|Components|CharacterMovement|SetMovementMode (Variables|/Script/Engine.Character|GetCharacterMovement (Game|GetPlayerCharacter 0)) "MOVE_Walking" 0)
    (Actor|DestroyActor)))

(fn ConstructionScript)